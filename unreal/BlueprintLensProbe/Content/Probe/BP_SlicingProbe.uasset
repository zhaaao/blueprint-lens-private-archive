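; BP_SlicingProbe is a small test-style Blueprint that exercises basic graph flow around a Health variable, with no evident gameplay role.
; On BeginPlay, a Sequence first applies a branch-guarded Health decrement, then calls the RunSecondaryPath custom event.
; That event waits on a short Delay, restores Health through the CalculateRecovery addition function, then runs a print loop.
; Overlap, Tick and the construction script are empty.
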(event `self.ReceiveBeginPlay`
  (`|ExecutionSequence`
    (:`then_0`
      (if (> (`self.Health`) 0)
        (set `self.Health` (- (`self.Health`) 10))
        (`KismetSystemLibrary.PrintString` "Health decreased")
        (else
          (`KismetSystemLibrary.PrintString` "Health depleted"))))
    (:`then_1`
      (`self.RunSecondaryPath`))))

(event `RunSecondaryPath`
  (`KismetSystemLibrary.Delay` 0.2)
  (set `self.Health` (`self.CalculateRecovery` (`self.Health`) 5))
  (`KismetSystemLibrary.PrintString` "Secondary path completed")
  (for _ (range 3)
    (`KismetSystemLibrary.PrintString` "Loop iteration"))
  (`KismetSystemLibrary.PrintString` "Loop completed"))

(fn `CalculateRecovery`
  (params (CurrentHealth :type Integer) (Bonus :type Integer))
  (returns (NewHealth :type Integer))
  (return (+ CurrentHealth Bonus)))

(fn `UserConstructionScript`)