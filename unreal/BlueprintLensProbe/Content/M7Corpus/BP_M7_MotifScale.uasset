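; BP_M7_MotifScale is a synthetic Blueprint that repeats graph motifs at scale in one M7_MOTIF_SCALE event, apparently as a test corpus asset.
; Nested Sequences hold branch-and-merge chains that set flags and print markers, plus long runs assigning the same two-counter sum.
; Each chain ends in a cyclic exec loop on a constant-true Branch, so the first loop never exits and its Delay branch is unreachable.
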(event `M7_MOTIF_SCALE`
  (bind _returnvalue (+ (`self.M7Counter000`) (`self.M7Counter001`)))
  (bind _returnvalue_2 (+ (`self.M7Counter000`) (`self.M7Counter001`)))
  (bind _returnvalue_3 (+ (`self.M7Counter000`) (`self.M7Counter001`)))
  (bind _returnvalue_4 (+ (`self.M7Counter000`) (`self.M7Counter001`)))
  (bind _returnvalue_5 (+ (`self.M7Counter000`) (`self.M7Counter001`)))
  (bind _returnvalue_6 (+ (`self.M7Counter000`) (`self.M7Counter001`)))
  (bind _returnvalue_7 (+ (`self.M7Counter000`) (`self.M7Counter001`)))
  (bind _returnvalue_8 (+ (`self.M7Counter000`) (`self.M7Counter001`)))
  (bind _returnvalue_9 (+ (`self.M7Counter000`) (`self.M7Counter001`)))
  (bind _returnvalue_10 (+ (`self.M7Counter000`) (`self.M7Counter001`)))
  (bind _returnvalue_11 (+ (`self.M7Counter000`) (`self.M7Counter001`)))
  (bind _returnvalue_12 (+ (`self.M7Counter000`) (`self.M7Counter001`)))
  (bind _returnvalue_13 (+ (`self.M7Counter000`) (`self.M7Counter001`)))
  (bind _returnvalue_14 (+ (`self.M7Counter000`) (`self.M7Counter001`)))
  (bind _returnvalue_15 (+ (`self.M7Counter000`) (`self.M7Counter001`)))
  (bind _returnvalue_16 (+ (`self.M7Counter000`) (`self.M7Counter001`)))
  (bind _returnvalue_17 (+ (`self.M7Counter000`) (`self.M7Counter001`)))
  (bind _returnvalue_18 (+ (`self.M7Counter000`) (`self.M7Counter001`)))
  (bind _returnvalue_19 (+ (`self.M7Counter000`) (`self.M7Counter001`)))
  (bind _returnvalue_20 (+ (`self.M7Counter000`) (`self.M7Counter001`)))
  (bind _returnvalue_21 (+ (`self.M7Counter000`) (`self.M7Counter001`)))
  (bind _returnvalue_22 (+ (`self.M7Counter000`) (`self.M7Counter001`)))
  (bind _returnvalue_23 (+ (`self.M7Counter000`) (`self.M7Counter001`)))
  (bind _returnvalue_24 (+ (`self.M7Counter000`) (`self.M7Counter001`)))
  (`|ExecutionSequence`
    (:`then_0`
      (`|ExecutionSequence`
        (:`then_0`
          (if true
            (set `self.M7Flag000` true)
            (else
              (set `self.M7Flag001` true)))
          (`KismetSystemLibrary.PrintString` "M7_BRANCH_MERGE_000")
          (if true
            (set `self.M7Flag002` true)
            (else
              (set `self.M7Flag003` true)))
          (`KismetSystemLibrary.PrintString` "M7_BRANCH_MERGE_001")
          (if true
            (set `self.M7Flag004` true)
            (else
              (set `self.M7Flag005` true)))
          (`KismetSystemLibrary.PrintString` "M7_BRANCH_MERGE_002")
          (if true
            (set `self.M7Flag006` true)
            (else
              (set `self.M7Flag007` true)))
          (`KismetSystemLibrary.PrintString` "M7_BRANCH_MERGE_003")
          (if true
            (set `self.M7Flag008` true)
            (else
              (set `self.M7Flag009` true)))
          (`KismetSystemLibrary.PrintString` "M7_BRANCH_MERGE_004")
          (if true
            (set `self.M7Flag010` true)
            (else
              (set `self.M7Flag011` true)))
          (`KismetSystemLibrary.PrintString` "M7_BRANCH_MERGE_005")
          (if true
            (set `self.M7Flag012` true)
            (else
              (set `self.M7Flag013` true)))
          (`KismetSystemLibrary.PrintString` "M7_BRANCH_MERGE_006")
          (if true
            (set `self.M7Flag014` true)
            (else
              (set `self.M7Flag015` true)))
          (`KismetSystemLibrary.PrintString` "M7_BRANCH_MERGE_007")
          (if true
            (set `self.M7Flag016` true)
            (else
              (set `self.M7Flag017` true)))
          (`KismetSystemLibrary.PrintString` "M7_BRANCH_MERGE_008")
          (if true
            (set `self.M7Flag018` true)
            (else
              (set `self.M7Flag019` true)))
          (`KismetSystemLibrary.PrintString` "M7_BRANCH_MERGE_009")
          (if true
            (set `self.M7Flag020` true)
            (else
              (set `self.M7Flag021` true)))
          (`KismetSystemLibrary.PrintString` "M7_BRANCH_MERGE_010")
          (if true
            (set `self.M7Flag022` true)
            (else
              (set `self.M7Flag023` true)))
          (`KismetSystemLibrary.PrintString` "M7_BRANCH_MERGE_011")
          (if true
            (set `self.M7Flag024` true)
            (else
              (set `self.M7Flag025` true)))
          (`KismetSystemLibrary.PrintString` "M7_BRANCH_MERGE_012")
          (if true
            (set `self.M7Flag026` true)
            (else
              (set `self.M7Flag027` true)))
          (`KismetSystemLibrary.PrintString` "M7_BRANCH_MERGE_013")
          (if true
            (set `self.M7Flag028` true)
            (else
              (set `self.M7Flag029` true)))
          (`KismetSystemLibrary.PrintString` "M7_BRANCH_MERGE_014")
          (if true
            (set `self.M7Flag030` true)
            (else
              (set `self.M7Flag031` true)))
          (`KismetSystemLibrary.PrintString` "M7_BRANCH_MERGE_015")
          (if true :!label _label
            (set `self.M7Flag064` true)
            (`KismetSystemLibrary.PrintString` "M7_SCC_00_CALL_00")
            (set `self.M7Flag065` true)
            (`KismetSystemLibrary.PrintString` "M7_SCC_00_CALL_01")
            (set `self.M7Flag066` true)
            (`KismetSystemLibrary.PrintString` "M7_SCC_00_CALL_02")
            (set `self.M7Flag067` true)
            (`KismetSystemLibrary.PrintString` "M7_SCC_00_CALL_03")
            (set `self.M7Flag068` true)
            (`KismetSystemLibrary.PrintString` "M7_SCC_00_CALL_04")
            (set `self.M7Flag069` true)
            (`KismetSystemLibrary.PrintString` "M7_SCC_00_CALL_05")
            (goto _label)
            (else
              (`KismetSystemLibrary.Delay` 0.0)
              (set `self.M7Flag070` true))))
        (:`then_1`
          (`|ExecutionSequence`
            (:`then_0`
              (set `self.M7Counter002` _returnvalue)
              (set `self.M7Counter003` _returnvalue)
              (set `self.M7Counter004` _returnvalue)
              (set `self.M7Counter005` _returnvalue_2)
              (set `self.M7Counter006` _returnvalue_2)
              (set `self.M7Counter007` _returnvalue_2)
              (set `self.M7Counter008` _returnvalue_3)
              (set `self.M7Counter009` _returnvalue_3)
              (set `self.M7Counter010` _returnvalue_3)
              (set `self.M7Counter011` _returnvalue_4)
              (set `self.M7Counter012` _returnvalue_4)
              (set `self.M7Counter013` _returnvalue_4)
              (set `self.M7Counter014` _returnvalue_5)
              (set `self.M7Counter015` _returnvalue_5)
              (set `self.M7Counter016` _returnvalue_5)
              (set `self.M7Counter017` _returnvalue_6)
              (set `self.M7Counter018` _returnvalue_6)
              (set `self.M7Counter019` _returnvalue_6)
              (set `self.M7Counter020` _returnvalue_7)
              (set `self.M7Counter021` _returnvalue_7)
              (set `self.M7Counter022` _returnvalue_7)
              (set `self.M7Counter023` _returnvalue_8)
              (set `self.M7Counter024` _returnvalue_8)
              (set `self.M7Counter025` _returnvalue_8)
              (set `self.M7Counter026` _returnvalue_9)
              (set `self.M7Counter027` _returnvalue_9)
              (set `self.M7Counter028` _returnvalue_9)
              (set `self.M7Counter029` _returnvalue_10)
              (set `self.M7Counter030` _returnvalue_10)
              (set `self.M7Counter031` _returnvalue_10)
              (set `self.M7Counter032` _returnvalue_11)
              (set `self.M7Counter033` _returnvalue_11)
              (set `self.M7Counter034` _returnvalue_11)
              (set `self.M7Counter035` _returnvalue_12)
              (set `self.M7Counter036` _returnvalue_12)
              (set `self.M7Counter037` _returnvalue_12)
              (if true :!label _label_2
                (set `self.M7Flag072` true)
                (`KismetSystemLibrary.PrintString` "M7_SCC_01_CALL_00")
                (set `self.M7Flag073` true)
                (`KismetSystemLibrary.PrintString` "M7_SCC_01_CALL_01")
                (set `self.M7Flag074` true)
                (`KismetSystemLibrary.PrintString` "M7_SCC_01_CALL_02")
                (set `self.M7Flag075` true)
                (`KismetSystemLibrary.PrintString` "M7_SCC_01_CALL_03")
                (set `self.M7Flag076` true)
                (`KismetSystemLibrary.PrintString` "M7_SCC_01_CALL_04")
                (set `self.M7Flag077` true)
                (`KismetSystemLibrary.PrintString` "M7_SCC_01_CALL_05")
                (goto _label_2)
                (else
                  (`KismetSystemLibrary.Delay` 0.0)
                  (set `self.M7Flag078` true))))))))
    (:`then_1`
      (`|ExecutionSequence`
        (:`then_0`
          (if true
            (set `self.M7Flag032` true)
            (else
              (set `self.M7Flag033` true)))
          (`KismetSystemLibrary.PrintString` "M7_BRANCH_MERGE_000")
          (if true
            (set `self.M7Flag034` true)
            (else
              (set `self.M7Flag035` true)))
          (`KismetSystemLibrary.PrintString` "M7_BRANCH_MERGE_001")
          (if true
            (set `self.M7Flag036` true)
            (else
              (set `self.M7Flag037` true)))
          (`KismetSystemLibrary.PrintString` "M7_BRANCH_MERGE_002")
          (if true
            (set `self.M7Flag038` true)
            (else
              (set `self.M7Flag039` true)))
          (`KismetSystemLibrary.PrintString` "M7_BRANCH_MERGE_003")
          (if true
            (set `self.M7Flag040` true)
            (else
              (set `self.M7Flag041` true)))
          (`KismetSystemLibrary.PrintString` "M7_BRANCH_MERGE_004")
          (if true
            (set `self.M7Flag042` true)
            (else
              (set `self.M7Flag043` true)))
          (`KismetSystemLibrary.PrintString` "M7_BRANCH_MERGE_005")
          (if true
            (set `self.M7Flag044` true)
            (else
              (set `self.M7Flag045` true)))
          (`KismetSystemLibrary.PrintString` "M7_BRANCH_MERGE_006")
          (if true
            (set `self.M7Flag046` true)
            (else
              (set `self.M7Flag047` true)))
          (`KismetSystemLibrary.PrintString` "M7_BRANCH_MERGE_007")
          (if true
            (set `self.M7Flag048` true)
            (else
              (set `self.M7Flag049` true)))
          (`KismetSystemLibrary.PrintString` "M7_BRANCH_MERGE_008")
          (if true
            (set `self.M7Flag050` true)
            (else
              (set `self.M7Flag051` true)))
          (`KismetSystemLibrary.PrintString` "M7_BRANCH_MERGE_009")
          (if true
            (set `self.M7Flag052` true)
            (else
              (set `self.M7Flag053` true)))
          (`KismetSystemLibrary.PrintString` "M7_BRANCH_MERGE_010")
          (if true
            (set `self.M7Flag054` true)
            (else
              (set `self.M7Flag055` true)))
          (`KismetSystemLibrary.PrintString` "M7_BRANCH_MERGE_011")
          (if true
            (set `self.M7Flag056` true)
            (else
              (set `self.M7Flag057` true)))
          (`KismetSystemLibrary.PrintString` "M7_BRANCH_MERGE_012")
          (if true
            (set `self.M7Flag058` true)
            (else
              (set `self.M7Flag059` true)))
          (`KismetSystemLibrary.PrintString` "M7_BRANCH_MERGE_013")
          (if true
            (set `self.M7Flag060` true)
            (else
              (set `self.M7Flag061` true)))
          (`KismetSystemLibrary.PrintString` "M7_BRANCH_MERGE_014")
          (if true
            (set `self.M7Flag062` true)
            (else
              (set `self.M7Flag063` true)))
          (`KismetSystemLibrary.PrintString` "M7_BRANCH_MERGE_015")
          (if true :!label _label_3
            (set `self.M7Flag080` true)
            (`KismetSystemLibrary.PrintString` "M7_SCC_02_CALL_00")
            (set `self.M7Flag081` true)
            (`KismetSystemLibrary.PrintString` "M7_SCC_02_CALL_01")
            (set `self.M7Flag082` true)
            (`KismetSystemLibrary.PrintString` "M7_SCC_02_CALL_02")
            (set `self.M7Flag083` true)
            (`KismetSystemLibrary.PrintString` "M7_SCC_02_CALL_03")
            (set `self.M7Flag084` true)
            (`KismetSystemLibrary.PrintString` "M7_SCC_02_CALL_04")
            (set `self.M7Flag085` true)
            (`KismetSystemLibrary.PrintString` "M7_SCC_02_CALL_05")
            (goto _label_3)
            (else
              (`KismetSystemLibrary.Delay` 0.0)
              (set `self.M7Flag086` true))))
        (:`then_1`
          (`|ExecutionSequence`
            (:`then_0`
              (set `self.M7Counter038` _returnvalue_13)
              (set `self.M7Counter039` _returnvalue_13)
              (set `self.M7Counter040` _returnvalue_13)
              (set `self.M7Counter041` _returnvalue_14)
              (set `self.M7Counter042` _returnvalue_14)
              (set `self.M7Counter043` _returnvalue_14)
              (set `self.M7Counter044` _returnvalue_15)
              (set `self.M7Counter045` _returnvalue_15)
              (set `self.M7Counter046` _returnvalue_15)
              (set `self.M7Counter047` _returnvalue_16)
              (set `self.M7Counter048` _returnvalue_16)
              (set `self.M7Counter049` _returnvalue_16)
              (set `self.M7Counter050` _returnvalue_17)
              (set `self.M7Counter051` _returnvalue_17)
              (set `self.M7Counter052` _returnvalue_17)
              (set `self.M7Counter053` _returnvalue_18)
              (set `self.M7Counter054` _returnvalue_18)
              (set `self.M7Counter055` _returnvalue_18)
              (set `self.M7Counter056` _returnvalue_19)
              (set `self.M7Counter057` _returnvalue_19)
              (set `self.M7Counter058` _returnvalue_19)
              (set `self.M7Counter059` _returnvalue_20)
              (set `self.M7Counter060` _returnvalue_20)
              (set `self.M7Counter061` _returnvalue_20)
              (set `self.M7Counter062` _returnvalue_21)
              (set `self.M7Counter063` _returnvalue_21)
              (set `self.M7Counter064` _returnvalue_21)
              (set `self.M7Counter065` _returnvalue_22)
              (set `self.M7Counter066` _returnvalue_22)
              (set `self.M7Counter067` _returnvalue_22)
              (set `self.M7Counter068` _returnvalue_23)
              (set `self.M7Counter069` _returnvalue_23)
              (set `self.M7Counter070` _returnvalue_23)
              (set `self.M7Counter071` _returnvalue_24)
              (set `self.M7Counter072` _returnvalue_24)
              (set `self.M7Counter073` _returnvalue_24)
              (if true :!label _label_4
                (set `self.M7Flag088` true)
                (`KismetSystemLibrary.PrintString` "M7_SCC_03_CALL_00")
                (set `self.M7Flag089` true)
                (`KismetSystemLibrary.PrintString` "M7_SCC_03_CALL_01")
                (set `self.M7Flag090` true)
                (`KismetSystemLibrary.PrintString` "M7_SCC_03_CALL_02")
                (set `self.M7Flag091` true)
                (`KismetSystemLibrary.PrintString` "M7_SCC_03_CALL_03")
                (set `self.M7Flag092` true)
                (`KismetSystemLibrary.PrintString` "M7_SCC_03_CALL_04")
                (set `self.M7Flag093` true)
                (`KismetSystemLibrary.PrintString` "M7_SCC_03_CALL_05")
                (goto _label_4)
                (else
                  (`KismetSystemLibrary.Delay` 0.0)
                  (set `self.M7Flag094` true))))))))))

(fn `UserConstructionScript`)