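; BP_LC1_LongChain is a Blueprint in the LensCorpus folder that consists of one long linear execution chain, with no visible gameplay behavior.
; On BeginPlay it sets a numbered series of step-completion booleans to true in order, then sets LC1Ready.
; The chain has no branches, delays or checks, so every flag is set in a single pass.
; Overlap and Tick are disabled placeholder events, and the construction script is empty.
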(event `self.ReceiveBeginPlay`
  (set `self.LC1Step01Complete` true)
  (set `self.LC1Step02Complete` true)
  (set `self.LC1Step03Complete` true)
  (set `self.LC1Step04Complete` true)
  (set `self.LC1Step05Complete` true)
  (set `self.LC1Step06Complete` true)
  (set `self.LC1Step07Complete` true)
  (set `self.LC1Step08Complete` true)
  (set `self.LC1Step09Complete` true)
  (set `self.LC1Step10Complete` true)
  (set `self.LC1Step11Complete` true)
  (set `self.LC1Step12Complete` true)
  (set `self.LC1Ready` true))

(fn `UserConstructionScript`)