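; BP_LC6_BoundaryMatrix is a Blueprint of four independent LC6 events named Opaque, Uncertain, Unsupported and Truncated, with no gameplay logic evident.
; Opaque prints a string and sets a done flag, while Unsupported sets its flag after a short latent Delay.
; Uncertain stores a select on a constant false condition, and Truncated sets a run of numbered flags.
; Nothing here calls the events or reads the variables, and the construction script is empty.
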(event `LC6_OPAQUE`
  (`KismetSystemLibrary.PrintString` "Hello")
  (set `self.LC6OpaqueDone` true))

(event `LC6_UNCERTAIN`
  (set `self.LC6UncertainResult` (select `bool` false :`true` true)))

(event `LC6_UNSUPPORTED`
  (`KismetSystemLibrary.Delay` 0.2)
  (set `self.LC6UnsupportedDone` true))

(event `LC6_TRUNCATED`
  (set `self.LC6Truncated01` true)
  (set `self.LC6Truncated02` true)
  (set `self.LC6Truncated03` true)
  (set `self.LC6Truncated04` true)
  (set `self.LC6Truncated05` true)
  (set `self.LC6Truncated06` true))

(fn `UserConstructionScript`)