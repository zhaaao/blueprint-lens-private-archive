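; BP_M10_CompositionDemo is a demo Blueprint of small graph-pattern cases, apparently a corpus for static graph analysis, with no gameplay logic.
; ComposedExecution combines a function call, Sequence, nested branches and an exitless back-edge; a separate Delay event joins its completion node.
; Other events isolate data producers, pure, impure and bodiless calls, a Select, and wired loops.
; ExitPresent increments its counter; ExitOutside never does, so its exit is unreachable.
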(event `DemoBodyUnavailable`
  (`KismetSystemLibrary.PrintString` "The event exists, but no same-named graph body exists."))

(event `ComposedExecution`
  (`self.DemoImpureBody`)
  (`|ExecutionSequence` :!label _label
    (:`then_0`
      (set `self.DataInputC` 0)
      (if (`self.OuterEnabled`)
        (if (`self.InnerEnabled`)
          (set `self.ComposedAccepted` true)
          (else
            (set `self.ComposedInnerRejected` true)))
        (else
          (set `self.ComposedOuterRejected` true)))
      (set `self.ComposedExecutionComplete` (> (`self.DataInputA`) (`self.DataInputB`)) :!label _label_2))
    (:`then_1`
      (set `self.DemoLoopCounter` 0)
      (set `self.DemoLoopVisited` true)
      (set `self.DemoLoopCounter` (+ (`self.DemoLoopCounter`) 1))
      (goto _label))
    (:`then_2`
      (`KismetSystemLibrary.PrintString` "Hello"))))

(event `ComposedUnsupportedBoundary`
  (`KismetSystemLibrary.Delay` 0.01)
  (goto _label_2))

(event `DataWithProducers`
  (set `self.DataWithProducersAnswer` (+ (+ (`self.DataInputA`) (`self.DataInputB`)) (`self.DataInputC`))))

(event `DataWithoutProducer`
  (set `self.DataWithoutProducerAnswer` true))

(event `LC5PureBody`
  (set `self.PureBodyAnswer` (`self.DemoPureBody`)))

(event `LC5ImpureBody`
  (`self.DemoImpureBody`)
  (set `self.ImpureBodyComplete` true))

(event `LC5BodyUnavailable`
  (`self.DemoBodyUnavailable`)
  (set `self.BodyUnavailableComplete` true))

(event `LC6Uncertain`
  (set `self.BoundaryComplete` (select `bool` (`self.OuterEnabled`) :`false` true :`true` false)))

(event `LC7ExitPresent`
  (set `self.ExitPresentCounter` 0)
  (if (< (`self.ExitPresentCounter`) 3) :!label _label_3
    (set `self.ExitPresentVisited` true)
    (set `self.ExitPresentCounter` (+ (`self.ExitPresentCounter`) 1))
    (goto _label_3)
    (else
      (set `self.ExitPresentComplete` true))))

(event `LC7ExitOutside`
  (set `self.ExitOutsideCounter` 0)
  (if (< (`self.ExitOutsideCounter`) 3) :!label _label_4
    (set `self.ExitOutsideVisited` true)
    (set `self.ExitOutsideComplete` true)
    (goto _label_4)
    (else
      (`KismetSystemLibrary.PrintString` "Exit exists beyond the selected static slice."))))

(fn `DataWithMultipleSets`
  (set `self.DataWithMultipleSetsAnswer` (+ (`self.DataInputA`) (`self.DataInputB`)))
  (set `self.DataWithMultipleSetsAnswer` (+ (`self.DataWithMultipleSetsAnswer`) (`self.DataInputC`))))

(fn `DemoImpureBody`
  (set `self.ImpureStage01` true)
  (set `self.ImpureStage02` true)
  (set `self.ImpureStage03` true)
  (set `self.ImpureStage04` true)
  (set `self.ImpureStage05` true)
  (set `self.ImpureStage06` true)
  (set `self.ImpureStage07` true)
  (set `self.ImpureStage08` true)
  (set `self.ImpureStage09` true)
  (set `self.ImpureStage10` true)
  (set `self.ImpureStage11` true)
  (set `self.ImpureStage12` true)
  (set `self.ImpureStage13` true)
  (set `self.ImpureStage14` true)
  (set `self.ImpureStage15` true))

(fn `DemoPureBody`
  (returns (Result :type Integer))
  (return (`self.DataInputA`)))

(fn `UserConstructionScript`)