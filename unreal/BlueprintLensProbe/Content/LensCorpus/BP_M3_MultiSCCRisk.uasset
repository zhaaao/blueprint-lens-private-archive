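; BP_M3_MultiSCCRisk is a Blueprint that models a parcel workflow as a flag-setting state sequence in one custom event.
; A priority check sets a route flag, then both paths continue into intake, validation and dispatch stages.
; Each stage loops back on itself through exec wires until its attempt counter reaches two, forming three separate cycles in series.
; Only dispatch recovery prints a message, and its acceptance marks the parcel complete.
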(event `M3_PARCEL_WORKFLOW`
  (set `self.M3WorkflowStarted` true)
  (if (`self.M3PriorityParcel`)
    (set `self.M3PriorityRoute` true)
    (else
      (set `self.M3StandardRoute` true)))
  (set `self.M3IntakeReady` true)
  (if (< (`self.M3IntakeAttempts`) 2) :!label _label
    (set `self.M3IntakeRetry` true)
    (set `self.M3IntakeAttempts` (+ (`self.M3IntakeAttempts`) 1))
    (goto _label)
    (else
      (set `self.M3IntakeAccepted` true)
      (if (< (`self.M3ValidationAttempts`) 2) :!label _label_2
        (set `self.M3ValidationRework` true)
        (set `self.M3ValidationAttempts` (+ (`self.M3ValidationAttempts`) 1))
        (goto _label_2)
        (else
          (set `self.M3ValidationAccepted` true)
          (if (< (`self.M3DispatchAttempts`) 2) :!label _label_3
            (`KismetSystemLibrary.PrintString` "Dispatch recovery remains opaque at core-v1")
            (set `self.M3DispatchRecovery` true)
            (set `self.M3DispatchAttempts` (+ (`self.M3DispatchAttempts`) 1))
            (goto _label_3)
            (else
              (set `self.M3DispatchAccepted` true)
              (set `self.M3ParcelComplete` true))))))))

(fn `UserConstructionScript`)