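; BP_LensCorpus_Main is an encounter Blueprint that appears to be a test sample, with placeholder logic and debug prints.
; BeginPlay runs a sequence: RunEncounter sets stage flags, a delayed CallService forwards to ServiceRef, and a timer schedules HandleDeferredWork.
; EvaluateEncounter derives Ready from health and armor versus threat, then BeginPlay fires OnStateChanged.
; Overlap events only print, Tick is disabled, and ComputeReadiness and DispatchRequest are uncalled here.
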(event `self.ReceiveBeginPlay`
  (`|ExecutionSequence`
    (:`then_0`
      (`self.RunEncounter`))
    (:`then_1`
      (`KismetSystemLibrary.Delay` 0.2)
      (`self.CallService` 5))
    (:`then_2`
      (`KismetSystemLibrary.K2_SetTimer` null "HandleDeferredWork" 1.0)
      (bind _shouldproceed (`self.EvaluateEncounter` (`self.Health`) (`self.Armor`) (`self.Threat`)))
      (set `self.Ready` _shouldproceed)
      (`self.OnStateChanged` "Ready"))))

(event `self.CorpusTrigger.OnComponentBeginOverlap`
  (params (OverlappedComponent :type "PrimitiveComponent Object Reference") (OtherActor :type "Actor Object Reference") (OtherComp :type "PrimitiveComponent Object Reference") (OtherBodyIndex :type Integer) (bFromSweep :type Boolean) (SweepResult :type "HitResult Structure (by ref)"))
  (`KismetSystemLibrary.PrintString` "CorpusTrigger component overlap"))

(event `self.ReceiveActorBeginOverlap`
  (params (OtherActor :type "Actor Object Reference"))
  (`KismetSystemLibrary.PrintString` "Actor overlap received"))

(fn `CallService`
  (params (Demand :type Integer))
  (returns (Accepted :type Boolean))
  (bind _accepted (`/Game/LensCorpus/BP_LensCorpus_Service.CommitEncounter_0` (`self.ServiceRef`) Demand))
  (set `self.IsServiceAccepted` _accepted)
  (return _accepted))

(fn `ComputeReadiness`
  (params (Base :type Integer) (Bonus :type Integer))
  (returns (Score :type Integer))
  (bind _returnvalue (+ (+ Base Bonus) (`self.Armor`)))
  (set `self.MaxCapacity` _returnvalue)
  (return _returnvalue))

(fn `DispatchRequest`
  (params (Context :type String))
  (returns (Accepted :type Boolean))
  (bind _accepted (`/Game/LensCorpus/BPI_LensCorpusTarget.RequestAction` (`self.TargetRef`) Context))
  (return _accepted))

(fn `EvaluateEncounter`
  (params (HealthValue :type Integer) (ArmorValue :type Integer) (ThreatValue :type Integer))
  (returns (ShouldProceed :type Boolean))
  (if (> HealthValue 0)
    (if (>= ArmorValue ThreatValue)
      (set `self.Ready` true)
      (else
        (set `self.Ready` false)))
    (else
      (set `self.Ready` false)))
  (set `self.IsAlive` true)
  (return (`self.Ready`)))

(fn `HandleDeferredWork`
  (`KismetSystemLibrary.PrintString` "Deferred work")
  (set `self.RetryCount` 1))

(fn `RunEncounter`
  (set `self.Stage01Complete` true)
  (set `self.Stage02Complete` true)
  (set `self.Stage03Complete` true)
  (set `self.Stage04Complete` true)
  (set `self.Stage05Complete` true)
  (set `self.Stage06Complete` true)
  (set `self.Stage07Complete` true)
  (set `self.Stage08Complete` true)
  (set `self.Stage09Complete` true)
  (set `self.Stage10Complete` true)
  (set `self.Stage11Complete` true)
  (set `self.Stage12Complete` true)
  (for _ (range 3)
    (`KismetSystemLibrary.PrintString` "Loop body"))
  (`KismetSystemLibrary.PrintString` "Encounter run complete"))

(fn `UserConstructionScript`)