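; BP_LensCorpus_Service is a Blueprint service that reports a capacity and accepts encounter commits against it.
; BeginPlay sets the capacity, clears the commit count and flags the service as available.
; CommitEncounter0 overwrites the count with the requested demand and broadcasts OnEncounterCommitted, then returns whether demand fits capacity.
; The broadcast fires even when demand exceeds capacity, and neither query nor commit checks availability.
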(event `self.ReceiveBeginPlay`
  (set `self.Capacity` 8)
  (set `self.CommitCount` 0)
  (set `self.IsAvailable` true))

(fn `CommitEncounter_0`
  (params (Demand :type Integer))
  (returns (Accepted :type Boolean))
  (bind _output_get (set `self.CommitCount` Demand))
  (`self.OnEncounterCommitted` _output_get)
  (return (<= Demand (`self.Capacity`))))

(fn `QueryCapacity_0`
  (returns (AvailableCapacity :type Integer))
  (return (`self.Capacity`)))

(fn `UserConstructionScript`)